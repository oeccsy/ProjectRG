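; BP_Sky is a sky actor that produces a brief lightning flash by toggling the level's sky light.
; On BeginPlay it finds the first actor tagged "SkyLight", casts it to a SkyLight and caches the reference.
; The OnThunder event makes that light's root component visible, waits a short delay, then hides it again.
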(event `self.ReceiveBeginPlay`
  (`self.BindSkyLight`))

(event `OnThunder`
  (`self.TurnOnLight`)
  (`KismetSystemLibrary.Delay` 0.2)
  (`self.TurnOffLight`))

(fn `BindSkyLight`
  (bind _outactors (`GameplayStatics.GetAllActorsWithTag` "SkyLight"))
  (bind _assky_light (cast `SkyLight` (`|GetArrayItem` _outactors)))
  (set `self.SkyLight` _assky_light))

(fn `TurnOffLight`
  (`SceneComponent.SetVisibility` (`Actor.RootComponent` (`self.SkyLight`)) false false))

(fn `TurnOnLight`
  (`SceneComponent.SetVisibility` (`Actor.RootComponent` (`self.SkyLight`)) true false))

(fn `UserConstructionScript`)