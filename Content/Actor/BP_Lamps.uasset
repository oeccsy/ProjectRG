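; Manager actor that switches the level's BP_Lamp_2 lamps off in three groups and back on all at once.
; BindLamps fills the Lamps array from actors tagged "Lamp2"; nothing in this Blueprint calls it.
; Each TurnOffGroup function covers a hardcoded index range, so group membership depends on the order the tag search returns.
; TurnOnAll loops over the whole array.
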(fn `BindLamps`
  (bind _outactors (`GameplayStatics.GetAllActorsWithTag` "Lamp2"))
  (for _array_element _outactors
    (bind _asbp_lamp_2 (cast `/Game/Assets/Modern_Gas_Station/Blueprints/BP_Lamp_2` _array_element))
    (`KismetArrayLibrary.Array_Add` (`self.Lamps`) _asbp_lamp_2)))

(fn `TurnOffGroup1`
  (for _index (range 5)
    (`/Game/Assets/Modern_Gas_Station/Blueprints/BP_Lamp_2.TurnOff` (`|GetArrayItem` (`self.Lamps`) _index))))

(fn `TurnOffGroup2`
  (for _index (range 5 11)
    (`/Game/Assets/Modern_Gas_Station/Blueprints/BP_Lamp_2.TurnOff` (`|GetArrayItem` (`self.Lamps`) _index))))

(fn `TurnOffGroup3`
  (for _index (range 11 17)
    (`/Game/Assets/Modern_Gas_Station/Blueprints/BP_Lamp_2.TurnOff` (`|GetArrayItem` (`self.Lamps`) _index))))

(fn `TurnOnAll`
  (for _array_element (`self.Lamps`)
    (`/Game/Assets/Modern_Gas_Station/Blueprints/BP_Lamp_2.TurnOn` _array_element)))

(fn `UserConstructionScript`)