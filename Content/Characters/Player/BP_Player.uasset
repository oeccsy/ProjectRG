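; Player character Blueprint that handles movement and tracks a punch and fire action state.
; BeginPlay registers the Enhanced Input mapping context, and IA_Move drives movement along the control rotation's right and forward vectors.
; Action functions set CurState, and UpdateState steps punch and waiting states one stage toward Idle per call, leaving fire states untouched.
; A helper sets global time dilation; neither it nor the state functions are called within this Blueprint.
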(event `self.ReceiveBeginPlay`
  (`self.BindIMC`))

(event `EnhancedInput|/Game/Inputs/Actions/IA_Move`
  (params (ActionValue :type "Vector2D Structure") (ElapsedSeconds :type "Float (double-precision)") (TriggeredSeconds :type "Float (double-precision)") (InputAction :type "InputAction Object Reference" :default "/Game/Inputs/Actions/IA_Move.IA_Move"))
  (:`Triggered`
    (`self.Move` ActionValue_X ActionValue_Y)))

(fn `BindIMC`
  (`EnhancedInputSubsystemInterface.AddMappingContext` (pcsubsystem `EnhancedInputLocalPlayerSubsystem` (`GameplayStatics.GetPlayerController` 0)) "/Game/Inputs/IMC_Player.IMC_Player" 0 (struct)))

(fn `CastFire`
  (set `self.CurState` "NewEnumerator8"))

(fn `CastPunch`
  (set `self.CurState` "NewEnumerator14"))

(fn `Fire`
  (set `self.CurState` "NewEnumerator9"))

(fn `Move`
  (params (InputVertical :type "Float (double-precision)") (InputHorizontal :type "Float (double-precision)"))
  (`self.AddMovementInput` (* (`KismetMathLibrary.GetRightVector` (`self.GetControlRotation`)) InputVertical))
  (`self.AddMovementInput` (* (`KismetMathLibrary.GetForwardVector` (`self.GetControlRotation`)) InputHorizontal)))

(fn `Punch`
  (set `self.CurState` "NewEnumerator11"))

(fn `SetTimeScale`
  (params (Scale :type "Float (double-precision)"))
  (`GameplayStatics.SetGlobalTimeDilation` Scale))

(fn `UpdateState`
  (switch `/Game/Characters/Player/EPlayerState` (`self.CurState`)
    (:`NewEnumerator10`
      (set `self.CurState` "NewEnumerator11"))
    (:`NewEnumerator14`
      (set `self.CurState` "NewEnumerator10"))
    (:`NewEnumerator11`
      (set `self.CurState` "NewEnumerator12"))
    (:`NewEnumerator12`
      (set `self.CurState` "NewEnumerator0"))
    (:`NewEnumerator13`
      (set `self.CurState` "NewEnumerator12"))))

(fn `UserConstructionScript`)