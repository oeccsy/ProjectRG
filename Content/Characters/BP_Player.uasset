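; BP_Player is a player character Blueprint that handles movement through Enhanced Input.
; On BeginPlay it adds the IMC_Player mapping context to player controller 0's input subsystem.
; IA_Move feeds Move, where X drives the control rotation's right vector and Y its forward vector, despite the swapped-sounding Vertical/Horizontal parameter names.
; Both directions use the full control rotation rather than yaw alone.
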(event `self.ReceiveBeginPlay`
  (`self.BindIMC`))

(event `EnhancedInput|/Game/Inputs/Actions/IA_Move`
  (params (ActionValue :type "Vector2D Structure") (ElapsedSeconds :type "Float (double-precision)") (TriggeredSeconds :type "Float (double-precision)") (InputAction :type "InputAction Object Reference" :default "/Game/Inputs/Actions/IA_Move.IA_Move"))
  (:`Triggered`
    (`self.Move` ActionValue_X ActionValue_Y)))

(fn `BindIMC`
  (`EnhancedInputSubsystemInterface.AddMappingContext` (pcsubsystem `EnhancedInputLocalPlayerSubsystem` (`GameplayStatics.GetPlayerController` 0)) "/Game/Inputs/IMC_Player.IMC_Player" 0 (struct)))

(fn `Move`
  (params (InputVertical :type "Float (double-precision)") (InputHorizontal :type "Float (double-precision)"))
  (`self.AddMovementInput` (* (`KismetMathLibrary.GetRightVector` (`self.GetControlRotation`)) InputVertical))
  (`self.AddMovementInput` (* (`KismetMathLibrary.GetForwardVector` (`self.GetControlRotation`)) InputHorizontal)))

(fn `UserConstructionScript`)