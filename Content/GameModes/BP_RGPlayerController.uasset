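; BP_RGPlayerController is the player controller for what appears to be a rhythm game, routing note-hit input to game mode systems.
; On BeginPlay it caches BP_RGGameMode and adds the player Enhanced Input mapping context.
; The A input adds a note to the note combination system and refreshes its widget, while S starts music through the music player system.
; The D input is unimplemented.
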(event `self.ReceiveBeginPlay`
  (`self.CacheGameMode`)
  (`self.BindIMC`))

(event `EnhancedInput|/Game/Inputs/Actions/IA_HitNoteA`
  (params (ActionValue :type Boolean) (ElapsedSeconds :type "Float (double-precision)") (TriggeredSeconds :type "Float (double-precision)") (InputAction :type "InputAction Object Reference" :default "/Game/Inputs/Actions/IA_HitNoteA.IA_HitNoteA"))
  (bind _notecombsystem (`/Game/GameModes/BP_RGGameMode.NoteCombSystem` (`self.GameMode`)))
  (:`Triggered`
    (`/Game/System/BP_NoteCombSystem.TryAddNoteA` _notecombsystem)
    (`/Game/System/BP_NoteCombSystem.UpdateCurNoteCombWidget` _notecombsystem)))

(event `EnhancedInput|/Game/Inputs/Actions/IA_HitNoteS`
  (params (ActionValue :type Boolean) (ElapsedSeconds :type "Float (double-precision)") (TriggeredSeconds :type "Float (double-precision)") (InputAction :type "InputAction Object Reference" :default "/Game/Inputs/Actions/IA_HitNoteS.IA_HitNoteS"))
  (:`Triggered`
    (`/Game/System/BP_MusicPlayerSystem.StartMusic` (`/Game/GameModes/BP_RGGameMode.MusicPlayerSystem` (`self.GameMode`)))))

(event `EnhancedInput|/Game/Inputs/Actions/IA_HitNoteD`
  (params (ActionValue :type Boolean) (ElapsedSeconds :type "Float (double-precision)") (TriggeredSeconds :type "Float (double-precision)") (InputAction :type "InputAction Object Reference" :default "/Game/Inputs/Actions/IA_HitNoteD.IA_HitNoteD")))

(fn `BindIMC`
  (`EnhancedInputSubsystemInterface.AddMappingContext` (pcsubsystem `EnhancedInputLocalPlayerSubsystem` (`GameplayStatics.GetPlayerController` 0)) "/Game/Inputs/IMC_Player.IMC_Player" 0 (struct)))

(fn `CacheGameMode`
  (bind _asbp_rggame_mode (cast `/Game/GameModes/BP_RGGameMode` (`GameplayStatics.GetGameMode`)))
  (set `self.GameMode` _asbp_rggame_mode))

(fn `UserConstructionScript`)