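; BP_RGGameMode is a game mode that creates the music and note comb systems when play begins.
; InitActors spawns BP_MusicPlayerSystem and BP_NoteCombSystem at the world origin and stores a reference to each.
; It then binds an event to the music player's OnNewBeatBegin dispatcher, though the bound handler is not shown here.
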(event `self.ReceiveBeginPlay`
  (`self.InitActors`))

(fn `InitActors`
  (bind _returnvalue (`|SpawnActorFromClass` "/Game/System/BP_MusicPlayerSystem.BP_MusicPlayerSystem_C" (`KismetMathLibrary.Conv_VectorToTransform` (0.0 0.0 0.0)) "Undefined" "MultiplyWithRoot" null null))
  (set `self.MusicPlayerSystem` _returnvalue)
  (bind _returnvalue_2 (`|SpawnActorFromClass` "/Game/System/BP_NoteCombSystem.BP_NoteCombSystem_C" (`KismetMathLibrary.Conv_VectorToTransform` (0.0 0.0 0.0)) "Undefined" "MultiplyWithRoot" null null))
  (set `self.NoteCombSystem` _returnvalue_2)
  (add `/Game/System/BP_MusicPlayerSystem.OnNewBeatBegin` (`self.MusicPlayerSystem`) (`|CreateDelegate` (`self.NoteCombSystem`) :!event `ClearNoteComb`)))

(fn `UserConstructionScript`)