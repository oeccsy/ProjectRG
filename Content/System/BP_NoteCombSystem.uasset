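; BP_NoteCombSystem is an actor that manages a string-based note combination and its on-screen display.
; On BeginPlay it enables input, adds the IMC_Player mapping context and creates the WBP_NoteComb widget.
; Helper functions append "A" to the combination, push it to the widget or clear both.
; The S and D note functions are empty stubs, and no input events call the helpers here.
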(event `self.ReceiveBeginPlay`
  (`self.BindIMC`)
  (`self.InitWidget`))

(fn `BindIMC`
  (bind _returnvalue (`GameplayStatics.GetPlayerController` 0))
  (`self.EnableInput` _returnvalue)
  (message `EnhancedInputSubsystemInterface.AddMappingContext` _returnvalue "/Game/Inputs/IMC_Player.IMC_Player" 0 (struct)))

(fn `ClearNoteComb`
  (set `self.CurNoteComb` "")
  (`self.UpdateCurNoteCombWidget`))

(fn `InitWidget`
  (bind _returnvalue (`|CreateWidget` "/Game/UI/WBP_NoteComb.WBP_NoteComb_C"))
  (bind _output_get (set `self.NoteCombWidget` _returnvalue))
  (`UserWidget.AddToViewport` _output_get 0))

(fn `TryAddNoteA`
  (set `self.CurNoteComb` (`KismetStringLibrary.Concat_StrStr` (`self.CurNoteComb`) "A")))

(fn `TryAddNoteD`)

(fn `TryAddNoteS`)

(fn `UpdateCurNoteCombWidget`
  (`/Game/UI/WBP_NoteComb.SetNoteText` (`self.NoteCombWidget`) (`KismetTextLibrary.Conv_StringToText` (`self.CurNoteComb`))))

(fn `UserConstructionScript`)