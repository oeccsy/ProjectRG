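; Legacy rhythm-input system that builds a per-beat string of note presses and shows it in an on-screen WBP_NoteComb widget.
; TryAddNoteA snaps offset-adjusted music time to one of eight beat slots, appending "A" to the current or next beat's combo, or failing it if the slot is taken.
; SwitchNoteComb promotes the next combo and refreshes the widget, red on failure.
; S and D handlers are empty stubs, and Threshold is unused.
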(event `self.ReceiveBeginPlay`
  (`self.InitWidget`))

(fn `AddComma`)

(fn `InitWidget`
  (bind _returnvalue (`|CreateWidget` "/Game/UI/WBP_NoteComb.WBP_NoteComb_C"))
  (bind _output_get (set `self.NoteCombWidget` _returnvalue))
  (`UserWidget.AddToViewport` _output_get 0))

(fn `SwitchNoteComb`
  (set `self.CurBeatCombData` (`self.NextBeatCombData`))
  (set `self.NextBeatCombData` (make `/Game/System/Data/NoteCombData` "" true (`|MakeArray` false false false false false false false false)))
  (`self.UpdateCurNoteCombWidget`))

(fn `TryAddNoteA`
  (params (MusicElapsedTime :type "Float (double-precision)") (CurBeatData :type "/Game/System/Data/BeatData Structure") (Threshold :type "Float (double-precision)"))
  (locals (`Note Index` :type Integer) (InputTime :type "Float (double-precision)"))
  (bind (_curbeatcombdata_comb _curbeatcombdata_combsuccess _curbeatcombdata_isnoteused) (break `/Game/System/Data/NoteCombData` (`self.CurBeatCombData`)))
  (bind (_nextbeatcombdata_comb _nextbeatcombdata_combsuccess _nextbeatcombdata_isnoteused) (break `/Game/System/Data/NoteCombData` (`self.NextBeatCombData`)))
  (bind (_nextbeatcombdata_comb_2 _nextbeatcombdata_combsuccess_2 _nextbeatcombdata_isnoteused_2) (break `/Game/System/Data/NoteCombData` (`self.NextBeatCombData`)))
  (bind (_curbeatcombdata_comb_2 _curbeatcombdata_combsuccess_2 _curbeatcombdata_isnoteused_2) (break `/Game/System/Data/NoteCombData` (`self.CurBeatCombData`)))
  (bind (_curbeatcombdata_comb_3 _curbeatcombdata_combsuccess_3 _curbeatcombdata_isnoteused_3) (break `/Game/System/Data/NoteCombData` (`self.CurBeatCombData`)))
  (bind (_nextbeatcombdata_comb_3 _nextbeatcombdata_combsuccess_3 _nextbeatcombdata_isnoteused_3) (break `/Game/System/Data/NoteCombData` (`self.NextBeatCombData`)))
  (bind (_curbeatcombdata_comb_4 _curbeatcombdata_combsuccess_4) (break `/Game/System/Data/NoteCombData` (`self.CurBeatCombData`)))
  (bind (_nextbeatcombdata_comb_4 _nextbeatcombdata_combsuccess_4) (break `/Game/System/Data/NoteCombData` (`self.NextBeatCombData`)))
  (bind (_curbeatcombdata_comb_5 _curbeatcombdata_combsuccess_5 _curbeatcombdata_isnoteused_4) (break `/Game/System/Data/NoteCombData` (`self.CurBeatCombData`)))
  (bind (_nextbeatcombdata_comb_5 _nextbeatcombdata_combsuccess_5 _nextbeatcombdata_isnoteused_4) (break `/Game/System/Data/NoteCombData` (`self.NextBeatCombData`)))
  (bind (_curbeatdata_index _curbeatdata_beattime _curbeatdata_duration) (break `/Game/System/Data/BeatData` (`local.CurBeatData`)))
  ;[1 1 1] Calc Input Time
  (set `local.InputTime` (+ (`local.MusicElapsedTime`) (`self.InputOffset`)))
  ;[1 1 1] Find Node Index
  (set `local.Note Index` (`KismetMathLibrary.Round` (* (/ (- (`local.InputTime`) _curbeatdata_beattime) _curbeatdata_duration) 8)))
  (if (< (`local.Note Index`) 8)
    ;[1 1 1] Check Comb Data Enable
    (if _curbeatcombdata_combsuccess_4
      ;[1 1 1] Update Cur Comb Data
      (if (`|GetArrayItem` _curbeatcombdata_isnoteused (`local.Note Index`))
        (set `self.CurBeatCombData` (make `/Game/System/Data/NoteCombData` _curbeatcombdata_comb_3 false _curbeatcombdata_isnoteused_3))
        (else
          (set `self.CurBeatCombData` (make `/Game/System/Data/NoteCombData` (`KismetStringLibrary.Concat_StrStr` _curbeatcombdata_comb_5 "A") true _curbeatcombdata_isnoteused_4))
          (`KismetArrayLibrary.Array_Set` _curbeatcombdata_isnoteused_2 (`local.Note Index`) true)))
      (`KismetSystemLibrary.PrintString` (`KismetStringLibrary.Concat_StrStr` "Note Hit Index : " (`KismetStringLibrary.Conv_IntToString` (`local.Note Index`))) :!label _label)
      (return))
    (else
      ;[1 1 1] Check Comb Data Enable
      (if _nextbeatcombdata_combsuccess_4
        ;[1 1 1] Update Next Comb Data
        (if (`|GetArrayItem` _nextbeatcombdata_isnoteused (`local.Note Index`))
          (set `self.NextBeatCombData` (make `/Game/System/Data/NoteCombData` _nextbeatcombdata_comb_3 false _nextbeatcombdata_isnoteused_3))
          (goto _label)
          (else
            (set `self.NextBeatCombData` (make `/Game/System/Data/NoteCombData` (`KismetStringLibrary.Concat_StrStr` _nextbeatcombdata_comb_5 "A") true _nextbeatcombdata_isnoteused_4))
            (`KismetArrayLibrary.Array_Set` _nextbeatcombdata_isnoteused_2 (`local.Note Index`) true)
            (goto _label)))))))

(fn `TryAddNoteAPrev`
  (returns (Result :type Boolean)))

(fn `TryAddNoteD`)

(fn `TryAddNoteS`)

(fn `UpdateCurNoteCombWidget`
  (bind _curbeatcombdata_comb (break `/Game/System/Data/NoteCombData` (`self.CurBeatCombData`)))
  (bind _curbeatcombdata_comb_2 (break `/Game/System/Data/NoteCombData` (`self.CurBeatCombData`)))
  (bind (_curbeatcombdata_comb_3 _curbeatcombdata_combsuccess) (break `/Game/System/Data/NoteCombData` (`self.CurBeatCombData`)))
  (if _curbeatcombdata_combsuccess
    (`/Game/UI/WBP_NoteComb.SetNoteText` (`self.NoteCombWidget`) (`KismetTextLibrary.Conv_StringToText` _curbeatcombdata_comb_2) (struct :`R` 1.0 :`G` 1.0 :`B` 1.0 :`A` 1.0))
    (else
      (`/Game/UI/WBP_NoteComb.SetNoteText` (`self.NoteCombWidget`) (`KismetTextLibrary.Conv_StringToText` _curbeatcombdata_comb) (struct :`R` 1.0 :`A` 1.0)))))

(fn `UserConstructionScript`)