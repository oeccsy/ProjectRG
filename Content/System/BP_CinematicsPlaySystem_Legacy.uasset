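; Legacy cinematics manager that plays camera sequences for the player and an enemy, chosen by index or player state.
; BeginPlay creates one LevelSequence player, caches the player pawn and first "Enemy"-tagged actor, then fills maps linking keys to sequences and sequences to actors.
; Both play functions reuse that sequence actor, swapping the sequence and rebinding the mapped actor at runtime.
; Index playback also sets BP_Player's state to Waiting.
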(event `self.ReceiveBeginPlay`
  (`self.InitActors`)
  (`self.InitSeqData`))

(fn `InitActors`
  (bind _outactor (`LevelSequencePlayer.CreateLevelSequencePlayer` "/Game/Cinematics/Test/Closeup_LevelSequence.Closeup_LevelSequence"))
  (set `self.SeqActor` _outactor)
  (set `self.PlayerActor` (`GameplayStatics.GetPlayerPawn` 0))
  (bind _outactors (`GameplayStatics.GetAllActorsWithTag` "Enemy"))
  (set `self.EnemyActor` (`|GetArrayItem` _outactors)))

(fn `InitSeqData`
  (`|ExecutionSequence`
    (:`then_0`
      (`BlueprintMapLibrary.Map_Add` (`self.TargetSeqByIndex`) 0 "/Game/Cinematics/Overview/PlayerOverview_LevelSequence.PlayerOverview_LevelSequence")
      (`BlueprintMapLibrary.Map_Add` (`self.TargetActor`) "/Game/Cinematics/Overview/PlayerOverview_LevelSequence.PlayerOverview_LevelSequence" (`self.PlayerActor`)))
    (:`then_1`
      (`BlueprintMapLibrary.Map_Add` (`self.TargetSeqByIndex`) 2 "/Game/Cinematics/Overview/EnemyOverview_LevelSequence.EnemyOverview_LevelSequence")
      (`BlueprintMapLibrary.Map_Add` (`self.TargetActor`) "/Game/Cinematics/Overview/EnemyOverview_LevelSequence.EnemyOverview_LevelSequence" (`self.EnemyActor`)))
    (:`then_2`
      (`BlueprintMapLibrary.Map_Add` (`self.TargetSeqByState`) "NewEnumerator14" "/Game/Cinematics/Closeup/PlayerCast_LevelSequence.PlayerCast_LevelSequence")
      (`BlueprintMapLibrary.Map_Add` (`self.TargetActor`) "/Game/Cinematics/Closeup/PlayerCast_LevelSequence.PlayerCast_LevelSequence" (`self.PlayerActor`)))
    (:`then_3`
      (`BlueprintMapLibrary.Map_Add` (`self.TargetSeqByState`) "NewEnumerator11" "/Game/Cinematics/Closeup/PlayerPunch_LevelSequence.PlayerPunch_LevelSequence")
      (`BlueprintMapLibrary.Map_Add` (`self.TargetActor`) "/Game/Cinematics/Closeup/PlayerPunch_LevelSequence.PlayerPunch_LevelSequence" (`self.PlayerActor`)))
    (:`then_4`
      (`BlueprintMapLibrary.Map_Add` (`self.TargetSeqByState`) "NewEnumerator16" "/Game/Cinematics/Closeup/EnemyCloseup_LevelSequence.EnemyCloseup_LevelSequence")
      (`BlueprintMapLibrary.Map_Add` (`self.TargetActor`) "/Game/Cinematics/Closeup/EnemyCloseup_LevelSequence.EnemyCloseup_LevelSequence" (`self.EnemyActor`)))
    (:`then_5`
      (`BlueprintMapLibrary.Map_Add` (`self.TargetSeqByState`) "NewEnumerator19" "/Game/Cinematics/Far/PlayerPowerPunch_LevelSequence.PlayerPowerPunch_LevelSequence")
      (`BlueprintMapLibrary.Map_Add` (`self.TargetActor`) "/Game/Cinematics/Far/PlayerPowerPunch_LevelSequence.PlayerPowerPunch_LevelSequence" (`self.EnemyActor`)))))

(fn `IsSeqExist`
  (params (Index :type Integer))
  (returns (Result :type Boolean))
  (return (`.ReturnValue` (`BlueprintMapLibrary.Map_Find` (`self.TargetSeqByIndex`) Index))))

(fn `Play by PlayerState`
  (params (State :type "/Game/Characters/Player/EPlayerState Enum" :default "NewEnumerator0"))
  (bind (_value _returnvalue) (`BlueprintMapLibrary.Map_Find` (`self.TargetSeqByState`) State))
  (bind (_value_2 _returnvalue_2) (`BlueprintMapLibrary.Map_Find` (`self.TargetActor`) _value))
  (if _returnvalue
    (if _returnvalue_2
      (`MovieSceneSequencePlayer.Stop` (`LevelSequenceActor.SequencePlayer` (`self.SeqActor`)))
      (`LevelSequenceActor.SetSequence` (`self.SeqActor`) _value)
      (`LevelSequenceActor.SetBinding` (`self.SeqActor`) (`|GetSequenceBinding` null) (`|MakeArray` _value_2) false)
      (`MovieSceneSequencePlayer.Play` (`LevelSequenceActor.SequencePlayer` (`self.SeqActor`))))))

(fn `PlayByIndex`
  (params (Index :type Integer))
  (bind (_value _returnvalue) (`BlueprintMapLibrary.Map_Find` (`self.TargetSeqByIndex`) Index))
  (bind (_value_2 _returnvalue_2) (`BlueprintMapLibrary.Map_Find` (`self.TargetActor`) _value))
  (if _returnvalue
    (if _returnvalue_2
      (`MovieSceneSequencePlayer.Stop` (`LevelSequenceActor.SequencePlayer` (`self.SeqActor`)))
      (`LevelSequenceActor.SetSequence` (`self.SeqActor`) _value)
      (`LevelSequenceActor.SetBinding` (`self.SeqActor`) (`|GetSequenceBinding` null) (`|MakeArray` _value_2) false)
      (`MovieSceneSequencePlayer.Play` (`LevelSequenceActor.SequencePlayer` (`self.SeqActor`)))
      (bind _asbp_player (cast `/Game/Characters/Player/BP_Player` (`self.PlayerActor`)))
      (set `/Game/Characters/Player/BP_Player.CurState` "Waiting" _asbp_player))))

(fn `Test`
  (`MovieSceneSequencePlayer.Stop` (`LevelSequenceActor.SequencePlayer` (`self.SeqActor`)))
  (`LevelSequenceActor.SetSequence` (`self.SeqActor`) "/Game/Cinematics/Overview/PlayerOverview_LevelSequence.PlayerOverview_LevelSequence")
  (`LevelSequenceActor.SetBinding` (`self.SeqActor`) (`|GetSequenceBinding` null) (`|MakeArray` (`GameplayStatics.GetPlayerPawn` 0) :!type "Actor Object Reference") false)
  (`MovieSceneSequencePlayer.Play` (`LevelSequenceActor.SequencePlayer` (`self.SeqActor`))))

(fn `UserConstructionScript`)