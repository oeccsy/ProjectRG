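; BP_SkillExecuteSystem maps note combinations to skill actors and runs the matching skill.
; On BeginPlay, RegisterSkills spawns a punch skill actor and stores it in SkillTable under its note string.
; ExecuteSkill looks up the given combination and runs that skill only if its CheckSkillValid check passes.
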(event `self.ReceiveBeginPlay`
  (`self.RegisterSkills`))

(fn `ExecuteSkill`
  (params (NoteComb :type String))
  (bind (_value _returnvalue) (`BlueprintMapLibrary.Map_Find` (`self.SkillTable`) NoteComb))
  (if _returnvalue
    (bind _valid (`/Game/System/Skill/BP_SkillNode.CheckSkillValid` _value))
    (if _valid
      (`/Game/System/Skill/BP_SkillNode.ExecuteSkill` _value))))

(fn `RegisterSkills`
  (`|ExecutionSequence`
    (:`then_0`
      (bind _returnvalue (`|SpawnActorFromClass` "/Game/System/Skill/BP_PunchSkill.BP_PunchSkill_C" (`KismetMathLibrary.Conv_VectorToTransform` (0.0 0.0 0.0)) "Undefined" "MultiplyWithRoot" null null))
      (`BlueprintMapLibrary.Map_Add` (`self.SkillTable`) "AAAA" _returnvalue))))

(fn `UserConstructionScript`)