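; BP_MusicPlaySystem_Legacy plays a music track and raises timing events for each beat and note in sync with it.
; BeginPlay loads beat timings from a data table, and StartMusic starts the audio and records an offset start time.
; Tick compares elapsed game time against the current beat and note, advancing beats through the table and deriving notes as eighths of the current beat's duration.
; Each advance fires a begin event and prints debug text.
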(event `self.ReceiveBeginPlay`
  (`self.InitBeatData`))

(event `self.ReceiveTick`
  (params (DeltaSeconds :type "Float (single-precision)"))
  (`self.UpdateBeatInfo`)
  (`self.UpdateNoteInfo`))

(fn `InitBeatData`
  (locals (BeatDataTable :type "DataTable Object Reference" :default "/Script/Engine.DataTable'/Game/System/Data/ABeatData.ABeatData'"))
  (bind _outrownames (`DataTableFunctionLibrary.GetDataTableRowNames` (`local.BeatDataTable`)))
  (for _array_element _outrownames
    (bind _returnvalue (`|GetDataTableRow` (`local.BeatDataTable`) _array_element)
      (:`then`
        (`KismetArrayLibrary.Array_Add` (`self.BeatDataList`) _returnvalue)))))

(fn `StartMusic`
  (locals (Offset :type "Float (double-precision)" :default 0.3))
  (`AudioComponent.Play` (`self.Audio`) 0.0)
  (set `self.MusicStartTime` (+ (`KismetSystemLibrary.GetGameTimeInSeconds`) (`local.Offset`)))
  (set `self.MusicElapsedTime` 0.0)
  (set `self.CurBeatData` (make `/Game/System/Data/BeatData` -1))
  (set `self.CurNoteData` (make `/Game/System/Data/NoteData` -1)))

(fn `UpdateBeatInfo`
  (bind (_curbeatdata_index _curbeatdata_beattime) (break `/Game/System/Data/BeatData` (`self.CurBeatData`)))
  (bind (_curbeatdata_index_2 _curbeatdata_beattime_2 _curbeatdata_duration) (break `/Game/System/Data/BeatData` (`self.CurBeatData`)))
  (bind _curbeatdata_index_3 (break `/Game/System/Data/BeatData` (`self.CurBeatData`)))
  ;[1 1 1] Check Update Valid
  (if (> (`self.MusicStartTime`) 0.0)
    ;[1 1 1] Update Elapsed Time
    (set `self.MusicElapsedTime` (- (`KismetSystemLibrary.GetGameTimeInSeconds`) (`self.MusicStartTime`)))
    ;[1 1 1] Check Beat Advance
    (if (<= (+ _curbeatdata_beattime_2 _curbeatdata_duration) (`self.MusicElapsedTime`))
      ;[1 1 1] Update Beat
      (set `self.CurBeatData` (`|GetArrayItem` (`self.BeatDataList`) (+ _curbeatdata_index_3 1)))
      (`self.OnBeatBegin`)
      (`KismetSystemLibrary.PrintString` (`KismetStringLibrary.Concat_StrStr` "New Beat : " (`KismetStringLibrary.Conv_DoubleToString` _curbeatdata_beattime))))))

(fn `UpdateNoteInfo`
  (bind (_curnotedata_index _curnotedata_notetime) (break `/Game/System/Data/NoteData` (`self.CurNoteData`)))
  (bind (_curnotedata_index_2 _curnotedata_notetime_2 _curnotedata_duration) (break `/Game/System/Data/NoteData` (`self.CurNoteData`)))
  (bind (_curbeatdata_index _curbeatdata_beattime _curbeatdata_duration) (break `/Game/System/Data/BeatData` (`self.CurBeatData`)))
  (bind _curnotedata_index_3 (break `/Game/System/Data/NoteData` (`self.CurNoteData`)))
  (bind (_curnotedata_index_4 _curnotedata_notetime_3 _curnotedata_duration_2) (break `/Game/System/Data/NoteData` (`self.CurNoteData`)))
  ;[1 1 1] Check Update Valid
  (if (> (`self.MusicStartTime`) 0.0)
    ;[1 1 1] Update Elapsed Time
    (set `self.MusicElapsedTime` (- (`KismetSystemLibrary.GetGameTimeInSeconds`) (`self.MusicStartTime`)))
    ;[1 1 1] Check Note Advance
    (if (<= (+ _curnotedata_notetime_2 _curnotedata_duration) (`self.MusicElapsedTime`))
      ;[1 1 1] Update Note Info
      (set `self.CurNoteData` (make `/Game/System/Data/NoteData` (mod (+ _curnotedata_index_3 1) 8) (+ _curnotedata_notetime_3 _curnotedata_duration_2) (/ _curbeatdata_duration 8.0)))
      (`self.OnNoteBegin`)
      (`KismetSystemLibrary.PrintString` (`KismetStringLibrary.Conv_DoubleToString` _curnotedata_notetime)))))

(fn `UserConstructionScript`)